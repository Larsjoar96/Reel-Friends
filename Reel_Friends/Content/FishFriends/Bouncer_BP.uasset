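; Bouncer NPC sprite that checks whether the player has gathered enough friends and shows the end screen when they have.
; On box overlap, it compares the character's NumFriends to FriendsNeeded: an exact match opens EndScreen, while too few swaps the bouncer's sprite for the player.
; Ending any overlap restores the default sprite.
; A yaw-only camera billboard function exists, but its Tick call is disabled by a constant condition.
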(event `self.ReceiveBeginPlay`
  (bind _asbp_third_person_character (cast `/Game/ThirdPerson/Blueprints/BP_ThirdPersonCharacter` (`GameplayStatics.GetPlayerPawn` 0)))
  (set `self.As BP Third Person Character` _asbp_third_person_character))

(event `LookAtCamera`
  (bind (_returnvalue_roll _returnvalue_pitch _returnvalue_yaw) (`KismetMathLibrary.BreakRotator` (`SceneComponent.K2_GetComponentRotation` (`/Game/ThirdPerson/Blueprints/BP_ThirdPersonCharacter.FollowCamera` (`self.As BP Third Person Character`)))))
  (`SceneComponent.K2_SetWorldRotation` (`self.PaperSprite`) (`KismetMathLibrary.MakeRotator` 0.0 0.0 (.yaw (`KismetMathLibrary.MakeRotator` _returnvalue_roll _returnvalue_pitch (- _returnvalue_yaw 90.0)))) false false))

(event `self.ReceiveTick`
  (params (DeltaSeconds :type "Float (single-precision)"))
  (if (not true)
    (`self.LookAtCamera`)))

(event `self.box_0.OnComponentBeginOverlap`
  (params (OverlappedComponent :type "PrimitiveComponent Object Reference") (OtherActor :type "Actor Object Reference") (OtherComp :type "PrimitiveComponent Object Reference") (OtherBodyIndex :type Integer) (bFromSweep :type Boolean) (SweepResult :type "HitResult Structure (by ref)"))
  (bind _papersprite (`self.PaperSprite`))
  (bind _asbp_third_person_character (cast `/Game/ThirdPerson/Blueprints/BP_ThirdPersonCharacter` (`GameplayStatics.GetPlayerPawn` 0)))
  (`/Engine/EditorBlueprintResources/StandardMacros.CompareFloat` (`/Game/ThirdPerson/Blueprints/BP_ThirdPersonCharacter.NumFriends` _asbp_third_person_character) (`self.FriendsNeeded`)
    (:`==`
      (`PaperSpriteComponent.SetSprite` _papersprite "/Game/FishFriends/FishSprites/Bouncer_1_Sprite_0.Bouncer_1_Sprite_0")
      (bind _returnvalue (`|CreateWidget` "/Game/Menu/EndScreen.EndScreen_C"))
      (`UserWidget.AddToViewport` _returnvalue 0))
    (:`<`
      (if (== OtherActor (`self.As BP Third Person Character`))
        (`PaperSpriteComponent.SetSprite` _papersprite "/Game/FishFriends/FishSprites/Bouncer_1_Sprite_1.Bouncer_1_Sprite_1")))))

(event `self.box_0.OnComponentEndOverlap`
  (params (OverlappedComponent :type "PrimitiveComponent Object Reference") (OtherActor :type "Actor Object Reference") (OtherComp :type "PrimitiveComponent Object Reference") (OtherBodyIndex :type Integer))
  (if true
    (`PaperSpriteComponent.SetSprite` (`self.PaperSprite`) "/Game/FishFriends/FishSprites/Bouncer_1_Sprite_0.Bouncer_1_Sprite_0")))

(fn `UserConstructionScript`)