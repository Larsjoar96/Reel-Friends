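; BP_SoundTrigger1 is a music or sound trigger actor that pairs a Box volume with an Audio component.
; The audio fades in on BeginPlay and whenever the first player pawn begins overlapping the box, then fades out when that pawn leaves.
; All fades share the same short duration, and other overlapping actors are ignored.
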(event `self.ReceiveBeginPlay`
  (`AudioComponent.FadeIn` (`self.Audio`) 2.0 1.0 0.0 "Linear"))

(event `self.Box.OnComponentBeginOverlap`
  (params (OverlappedComponent :type "PrimitiveComponent Object Reference") (OtherActor :type "Actor Object Reference") (OtherComp :type "PrimitiveComponent Object Reference") (OtherBodyIndex :type Integer) (bFromSweep :type Boolean) (SweepResult :type "HitResult Structure (by ref)"))
  (if (== OtherActor (`GameplayStatics.GetPlayerPawn` 0))
    (`AudioComponent.FadeIn` (`self.Audio`) 2.0 1.0 0.0 "Linear")))

(event `self.Box.OnComponentEndOverlap`
  (params (OverlappedComponent :type "PrimitiveComponent Object Reference") (OtherActor :type "Actor Object Reference") (OtherComp :type "PrimitiveComponent Object Reference") (OtherBodyIndex :type Integer))
  (if (== OtherActor (`GameplayStatics.GetPlayerPawn` 0))
    (`AudioComponent.FadeOut` (`self.Audio`) 2.0 0.0 "Linear")))

(fn `UserConstructionScript`)